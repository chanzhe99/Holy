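; AI controller for enemy characters that runs each pawn's behavior tree and links it to a combat director.
; On BeginPlay it caches the enemy pawn, player target and first valid director, then starts the tree and writes the initial AIState to the blackboard.
; QueueAttack updates that state, and Command_Attack triggers the pawn's attack.
; On a death message it asks the director to handle the death and destroys the pawn only if approved.
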(event Custom|Command_Attack
  ;[1 1 1] Events
  (Default|TriggerAttack (Variables|Default|GetEnemyPawnReference)))

(event Custom|QueueAttack
  (bind _output_get (Variables|Default|SetCurrentState "NewEnumerator1"))
  (AI|Components|Blackboard|SetValueasEnum (AI|GetBlackboard 0) (Utilities|Name|MakeLiteralName "AIState") _output_get))

(event Custom|ReceiveMessage_Death
  ;[1 1 1] Events
  (bind _successfuldeath (CallFunction|RequestDirectorforAIDeath (Variables|Default|GetEnemyPawnReference)))
  (if _successfuldeath
    (CallFunction|DestroyPawn)))

(event EventBeginPlay
  (bind _returnvalue (AI|GetBlackboard 0))
  (Utilities|FlowControl|Sequence
    (:then_0
      ;[1 1 1] Cache pawn ref & Set current target
      (bind _asbp_enemy_cpp (Utilities|Casting|CastToBP_EnemyCpp (Pawn|GetControlledPawn)))
      (bind _output_get (Variables|Default|SetEnemyPawnReference _asbp_enemy_cpp))
      (Variables|Default|SetCurrentTarget (Game|GetPlayerCharacter 0))
      ;[1 1 1] Cache Director
      (bind _outactors (Actor|GetAllActorsOfClass (Variables|Default|GetCombatDirectorClassType)))
      (bind _array_element (Utilities|Array|ForEachLoopwithBreak _outactors :!label _label)
        (:LoopBody
          (Utilities|IsValid _array_element
            (:Is%20Valid
              (Variables|Default|SetCombatDirectorReference _array_element)
              (goto _label Break))))))
    (:then_1
      (AI|RunBehaviorTree (Variables|/Game/Characters/Enemies/Enemy_Clean/BP_EnemyCpp.BP_EnemyCpp_C|GetBehaviourTree _output_get)))
    (:then_2
      ;[1 1 1] Post blackboard initialisation
      ;;[1 1 1] Set Initial State value in Blackboard
      (Utilities|IsValid _returnvalue
        (:Is%20Valid
          (AI|Components|Blackboard|SetValueasEnum _returnvalue (Utilities|Name|MakeLiteralName "AIState") (Variables|Default|GetCurrentState)))))))

(fn ConstructionScript)

(fn RequestDirectorforAIDeath
  (params (Target :type BP%20Enemy%20Cpp%20Object%20Reference))
  (bind _combatdirectorreference (Variables|Default|GetCombatDirectorReference)
    (:then
      (bind _succesfuldeath (Default|HandleAIDeath _combatdirectorreference Target))
      (return _succesfuldeath))
    (:else)))

(fn DestroyPawn
  (Actor|DestroyActor (Variables|Default|GetEnemyPawnReference))
  (return))