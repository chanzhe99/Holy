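; Combat director that decides which spawned enemy attacks next, grading all enemies found at BeginPlay.
; A looping timer, much faster in OraOra mode, scales each random-seeded grade by how directly the enemy's facing opposes the camera's.
; The top-graded enemy's AI controller queues an attack, then its grade is re-randomised.
; HandleAIDeath removes enemies; the simultaneous-attack limit is unfinished and debug-widget setup is unwired.
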(event Custom|RequestControllerAttackEvent
  (CallFunction|RecalculateScores)
  (CallFunction|RequestControllerAttack))

(event EventBeginPlay
  (Utilities|FlowControl|Sequence
    (:then_0
      (CallFunction|InitialiseDirector)
      (CallFunction|ResetAIGrading))
    (:then_1
      (Utilities|Time|SetTimerbyEvent (delegate Custom|RequestControllerAttackEvent) (CallFunction|GetAttackInterval) true))))

(fn ConstructionScript)

(fn InitialiseDirector
  ;[1 1 1] This is temporary, for initial spawned units, or until we set up spawners
  (bind _outactors (Actor|GetAllActorsOfClass (Variables|AI|GetAIClass)))
  (for _array_element _outactors
    (Utilities|Array|Add (Variables|AI|GetAIList) _array_element)
    (bind _asbp_enemy_aicontroller (Utilities|Casting|CastToBP_EnemyAIController (AI|GetAIController _array_element)))
    (Variables|/Game/Characters/Enemies/AI/BP_EnemyAIController.BP_EnemyAIController_C|SetEnableOraOraMode _asbp_enemy_aicontroller (Variables|Default|GetEnableOraOraMode)))
  (Variables|Default|SetIsActive true)
  (return))

(fn ResetAIGrading
  (for _array_element (Variables|AI|GetAIList)
    (Utilities|Map|Add (Variables|AI|GetAIGrading) _array_element (Math|Random|RandomFloatinRange 1.0 5.0)))
  (return))

(fn InitialiseDebuggingInterface
  (for _array_element (Variables|AI|GetAIList)
    (bind _returnvalue (UserInterface|CreateWidget "/Game/Characters/Enemies/AI/WBP_Debug_BP_EnemyCpp.WBP_Debug_BP_EnemyCpp_C" 0 _array_element (.Value (Utilities|Map|Find (Variables|AI|GetAIGrading) _array_element))))
    (Utilities|Map|Add (Variables|AI|GetAIDebugWidgets) _array_element _returnvalue)
    (bind _returnvalue_2 (AddComponent|AddWidgetComponent _array_element false))
    (UserInterface|SetWidget _returnvalue_2 _returnvalue))
  (return))

(fn FindHighestGradedAI
  (bind _aigrading (Variables|AI|GetAIGrading))
  (Utilities|Array|Clear (LocalVariables|GetGradeList))
  (bind _keys (Utilities|Map|Keys _aigrading))
  (for _array_element _keys
    (if (> (.Value (Utilities|Map|Find _aigrading _array_element)) (LocalVariables|GetHighestValue))
      (bind _output_get (LocalVariables|SetHighestValue (.Value (Utilities|Map|Find _aigrading _array_element))))
      (LocalVariables|SetHighestGradedAI _array_element)
      (Utilities|Array|Add (LocalVariables|GetGradeList) _output_get)))
  (return (Utilities|Array|MakeArray (LocalVariables|GetHighestGradedAI))))

(fn RequestControllerAttack
  (bind _foundais (CallFunction|FindHighestGradedAI))
  (for _array_element _foundais
    (bind _asbp_enemy_aicontroller (Utilities|Casting|CastToBP_EnemyAIController (AI|GetAIController _array_element)))
    (Default|QueueAttack _asbp_enemy_aicontroller)
    (Utilities|Map|Add (Variables|AI|GetAIGrading) _array_element (Math|Random|RandomFloatinRange 1.0 5.0)))
  (return))

(fn UpdateDebugWidgetValue
  (params (AIInstance :type BP%20Enemy%20Cpp%20Object%20Reference))
  (if (> (Utilities|Map|Length (Variables|AI|GetAIDebugWidgets)) 0)
    (Variables|/Game/Characters/Enemies/AI/WBP_Debug_BP_EnemyCpp.WBP_Debug_BP_EnemyCpp_C|SetCombatGrade (.Value (Utilities|Map|Find (Variables|AI|GetAIDebugWidgets) AIInstance)) (.Value (Utilities|Map|Find (Variables|AI|GetAIGrading) AIInstance)))
    (return)))

(fn RecalculateScores
  (CallFunction|ScorebyPosition))

(fn ScorebyPosition
  (Utilities|Array|Clear (LocalVariables|GetScoreList))
  (for _array_element (Variables|AI|GetAIList)
    (LocalVariables|SetCurrentAI _array_element)
    (Utilities|Array|Add (LocalVariables|GetScoreList) (* (.Value (Utilities|Map|Find (Variables|AI|GetAIGrading) (LocalVariables|GetCurrentAI))) (+ (Math|Float|NormalizetoRange (* (Math|Vector|DotProduct (Transformation|GetActorForwardVector _array_element) (Math|Vector|GetForwardVector (Camera|GetCameraRotation (Game|GetPlayerCameraManager 0)))) -1.0) -1.0 1.0) 0.5)))
    (Utilities|Map|Add (Variables|AI|GetAIGrading) (LocalVariables|GetCurrentAI) (* (.Value (Utilities|Map|Find (Variables|AI|GetAIGrading) (LocalVariables|GetCurrentAI))) (+ (Math|Float|NormalizetoRange (* (Math|Vector|DotProduct (Transformation|GetActorForwardVector _array_element) (Math|Vector|GetForwardVector (Camera|GetCameraRotation (Game|GetPlayerCameraManager 0)))) -1.0) -1.0 1.0) 0.5)))
    (CallFunction|UpdateDebugWidgetValue (LocalVariables|GetCurrentAI)))
  (Utilities|Array|ForEachLoopwithBreak (LocalVariables|GetScoreList)
    (:LoopBody
      (bind _result (Math|Integer|IncrementInt (LocalVariables|GetCurrentAttacks))
        (:%20%20
          (if (<= _result (Variables|Default|GetNumberOfSimultaneousAttacksAllowed))
            _))))))

(fn Test-doesnotwork
  (bind _outarray (Class|UArrayBlueprintLibrary|QuickSort (Utilities|Array|MakeArray (Math|Random|RandomFloatinRange 0.0 1e+01) (Math|Random|RandomFloatinRange 0.0 1e+01) (Math|Random|RandomFloatinRange 0.0 1e+01) (Math|Random|RandomFloatinRange 0.0 1e+01) (Math|Random|RandomFloatinRange 0.0 1e+01))))
  (for _array_element _outarray
    (LocalVariables|SetPrintString (Utilities|String|Append (LocalVariables|GetPrintString) (Utilities|String|ToString(Float) _array_element) ", ")))
  (Development|PrintString (LocalVariables|GetPrintString) true true "(R=0.000000,G=0.660000,B=1.000000,A=1.000000)" 1e+04))

(fn HandleAIDeath
  (params (AI :type BP%20Enemy%20Cpp%20Object%20Reference))
  (bind _aidebugwidgets (Variables|AI|GetAIDebugWidgets))
  (bind _output_get (LocalVariables|SetTarget AI))
  (Utilities|IsValid _output_get
    (:Is%20Valid
      (Utilities|FlowControl|Sequence
        (:then_0
          (Utilities|Array|RemoveItem (Variables|AI|GetAIList) (LocalVariables|GetTarget)))
        (:then_1
          (Utilities|Map|Remove (Variables|AI|GetAIGrading) (LocalVariables|GetTarget)))
        (:then_2
          (if (> (Utilities|Map|Length _aidebugwidgets) 0)
            (Widget|RemovefromParent (.Value (Utilities|Map|Find _aidebugwidgets (LocalVariables|GetTarget))))
            (Utilities|Map|Remove (Variables|AI|GetAIDebugWidgets) (LocalVariables|GetTarget))))
        (:then_3
          (return true))))
    (:Is%20Not%20Valid
      (return false))))

(fn GetAttackInterval
  (if (Variables|Default|GetEnableOraOraMode)
    (return 0.25)
    (else
      (return 4.0))))