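; Base Blueprint for an enemy projectile that is launched through an activation call with a velocity and a damage value.
; On BeginPlay it makes the root scene component the one moved by its ProjectileMovement component, with rotation following velocity.
; ActivateProjectile stores the contact damage, enables movement ticking and applies the starting velocity.
; The graphs shown only store the damage, with no hit handling.
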(event EventBeginPlay
  (CallFunction|SetupDefaults))

(fn ConstructionScript)

(fn SetupDefaults
  (bind _projectilemovement (Variables|Default|GetProjectileMovement))
  (Components|Movement|SetUpdatedComponent _projectilemovement (Variables|Default|GetDefaultSceneRoot))
  (Variables|/Script/Engine.ProjectileMovementComponent|SetbRotationFollowsVelocity _projectilemovement true)
  (return))

(fn ActivateProjectile
  (params (StartingVelocity :type Vector) (Damage :type Integer))
  (bind _projectilemovement (Variables|Default|GetProjectileMovement))
  (Variables|Default|SetDamageOnContact Damage)
  (Components|Tick|SetComponentTickEnabled _projectilemovement true)
  (Variables|/Script/Engine.MovementComponent|SetVelocity _projectilemovement StartingVelocity)
  (return))