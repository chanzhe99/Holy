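; Enemy stone projectile that damages BP_Demon on contact and uses a bouncing projectile movement set up on BeginPlay.
; A demon overlap applies contact damage and cuts velocity to a small fraction, with a debug print.
; Any overlap also turns on sphere physics, then timers make it ignore Pawn collision shortly after and destroy it after DestroyTimeDelay.
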(event OnComponentBeginOverlap(Sphere)
  (params (OverlappedComponent :type Primitive%20Component%20Object%20Reference) (OtherActor :type Actor%20Object%20Reference) (OtherComp :type Primitive%20Component%20Object%20Reference) (OtherBodyIndex :type Integer) (bFromSweep :type Boolean) (SweepResult :type Hit%20Result%20Structure%20%28by%20ref%29))
  (bind _projectilemovement (Variables|Default|GetProjectileMovement))
  (Utilities|FlowControl|Sequence
    (:then_0
      (bind _asbp_demon (Utilities|Casting|CastToBP_Demon OtherActor))
      (Class|Demon|ApplyDamage _asbp_demon (Variables|Default|GetDamageOnContact))
      (Variables|/Script/Engine.MovementComponent|SetVelocity _projectilemovement (* (Variables|/Script/Engine.MovementComponent|GetVelocity _projectilemovement) 0.05))
      (Development|PrintString "eat stone"))
    (:then_1
      (Physics|SetSimulatePhysics (Variables|Default|GetSphere) true)
      (bind _returnvalue (Utilities|Time|SetTimerbyEvent (delegate Custom|OnHitEvent) 0.1))
      (Variables|Default|SetHitTimerHandle _returnvalue)
      (bind _returnvalue_2 (Utilities|Time|SetTimerbyEvent (delegate Custom|PostHitEvent) (Variables|Default|GetDestroyTimeDelay)))
      (Variables|Default|SetDestroyTimerHandle _returnvalue_2))))

(event Custom|OnHitEvent
  (Utilities|Time|ClearandInvalidateTimerbyHandle (Variables|Default|GetHitTimerHandle))
  (Collision|SetCollisionResponsetoChannel (Variables|Default|GetSphere) "ECC_Pawn" "ECR_Ignore"))

(event Custom|PostHitEvent
  (Utilities|Time|ClearandInvalidateTimerbyHandle (Variables|Default|GetDestroyTimerHandle))
  (Actor|DestroyActor))

(event EventBeginPlay
  (bind _projectilemovement (Variables|Default|GetProjectileMovement))
  (|CallParentFunction)
  (Variables|/Script/Engine.ProjectileMovementComponent|SetbShouldBounce _projectilemovement true)
  (Variables|/Script/Engine.ProjectileMovementComponent|SetbSimulationEnabled _projectilemovement true)
  (Variables|/Script/Engine.ProjectileMovementComponent|SetBounciness _projectilemovement 1e+02))

(fn ConstructionScript
  (|CallParentFunction))