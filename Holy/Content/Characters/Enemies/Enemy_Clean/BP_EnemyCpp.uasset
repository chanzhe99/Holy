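; Enemy character Blueprint that performs a melee punch against BP_Demon players and reports its death to BP_EnemyAIController.
; DoAttack plays the punch montage while chained timers open and close the PunchHitBox collision window, with the enable and disable delays scaled by animation speed.
; Overlap applies damage once, holding the hit player until end overlap to block repeat hits.
; Health reset, death check and notification helpers complete it.
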(event OnComponentBeginOverlap(PunchHitBox)
  (params (OverlappedComponent :type Primitive%20Component%20Object%20Reference) (OtherActor :type Actor%20Object%20Reference) (OtherComp :type Primitive%20Component%20Object%20Reference) (OtherBodyIndex :type Integer) (bFromSweep :type Boolean) (SweepResult :type Hit%20Result%20Structure%20%28by%20ref%29))
  ;[1 1 1] Handle Attack on Collision
  (bind _asbp_demon (Utilities|Casting|CastToBP_Demon OtherActor))
  (Utilities|IsValid (Variables|Default|GetAttackedPlayerReference)
    (:Is%20Not%20Valid
      (bind _output_get (Variables|Default|SetAttackedPlayerReference _asbp_demon))
      (Class|Demon|ApplyDamage _output_get (Variables|Default|GetAttackDamage))
      (if (Variables|/Game/Characters/Enemies/AI/BP_EnemyAIController.BP_EnemyAIController_C|GetEnableOraOraMode (Variables|Default|GetControllerReference))
        (Development|PrintString "MUDAMUDAMUDAMUDA" true true "(R=0.000000,G=0.660000,B=1.000000,A=1.000000)" 3.0)
        (else
          (Development|PrintString "Player attacked" true true "(R=0.000000,G=0.660000,B=1.000000,A=1.000000)" 1.0))))))

(event OnComponentEndOverlap(PunchHitBox)
  (params (OverlappedComponent :type Primitive%20Component%20Object%20Reference) (OtherActor :type Actor%20Object%20Reference) (OtherComp :type Primitive%20Component%20Object%20Reference) (OtherBodyIndex :type Integer))
  ;[1 1 1] Handle Attack on Collision
  (bind _asbp_demon (Utilities|Casting|CastToBP_Demon OtherActor))
  (if (== _asbp_demon (Variables|Default|GetAttackedPlayerReference))
    (Variables|Default|SetAttackedPlayerReference 0)))

(event Custom|HandleAttackCollision
  (params (SpeedRatio :type Float%20%28single-precision%29))
  ;[1 1 1] Attack Collision Enable/Disable Sequence
  (Utilities|Time|ClearandInvalidateTimerbyHandle (Variables|Default|GetAttackCollisionTimerHandle))
  (bind _returnvalue (Utilities|Time|SetTimerbyEvent (delegate Custom|EnableAttackCollision_LocalEvent) (/ (Variables|Default|GetAttackCollisionEnableDelay) SpeedRatio)))
  (Variables|Default|SetAttackCollisionTimerHandle _returnvalue))

(event Custom|EnableAttackCollision_LocalEvent
  ;[1 1 1] Attack Collision Enable/Disable Sequence
  (Utilities|Time|ClearandInvalidateTimerbyHandle (Variables|Default|GetAttackCollisionTimerHandle))
  (Collision|SetCollisionEnabled (Variables|Default|GetPunchHitBox) "QueryOnly")
  (bind _returnvalue (Utilities|Time|SetTimerbyEvent (delegate Custom|DisableAttackCollision_LocalEvent) (/ (Variables|Default|GetAttackCollisionDisableDelay) (stale Custom|HandleAttackCollision SpeedRatio))))
  (Variables|Default|SetAttackCollisionTimerHandle _returnvalue))

(event Custom|DisableAttackCollision_LocalEvent
  ;[1 1 1] Attack Collision Enable/Disable Sequence
  (Utilities|Time|ClearandInvalidateTimerbyHandle (Variables|Default|GetAttackCollisionTimerHandle))
  (Collision|SetCollisionEnabled (Variables|Default|GetPunchHitBox) "NoCollision"))

(event EventBeginPlay
  (Utilities|FlowControl|Sequence
    (:then_0
      (bind _asbp_enemy_aicontroller (Utilities|Casting|CastToBP_EnemyAIController (AI|GetAIController self)))
      (Variables|Default|SetControllerReference _asbp_enemy_aicontroller)
      (CallFunction|ResetHealth))
    (:then_1
      (Variables|Default|SetIsReady true))))

(event EventSendDeathNotification
  (CallFunction|NotifyDeathtoController))

(fn ConstructionScript)

(fn DoAttack
  (params (AnimSpeedRatio :type Float%20%28single-precision%29))
  (Utilities|FlowControl|Sequence
    (:then_0
      (Animation|PlayAnimMontage "/Game/Characters/Enemies/Enemy_Clean/Animations/WidePunchAnimMontage.WidePunchAnimMontage" AnimSpeedRatio "None"))
    (:then_1
      (CallFunction|HandleAttackCollision AnimSpeedRatio))))

(fn ResetHealth
  (Variables|Default|SetEnemyHP (Variables|Default|GetMaxHealth))
  (return))

(fn CheckHealthStatus
  (return (<= (Variables|Default|GetEnemyHP) 0)))

(fn NotifyDeathtoController
  (Default|ReceiveMessageDeath (Variables|Default|GetControllerReference)))