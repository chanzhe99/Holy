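; BP_RangedEnemy is an enemy character that attacks by firing projectiles at the player.
; Its attack sequence starts a timer, with the delay scaled by the speed ratio, that spawns the projectile class at a spawn point with itself as instigator.
; The projectile is activated with attack damage and a straight-line velocity aimed slightly above the player's location at the moment of firing.
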(event Custom|SpawnProjectile_LocalEvent
  ;[1 1 1] Attack Sequence : Spawn projectile
  (Utilities|Time|ClearandInvalidateTimerbyHandle (Variables|Default|GetAttackSequenceTimerHandle))
  (bind _returnvalue (Game|SpawnActorfromClass (Variables|Default|GetProjectileClass) (Transformation|GetWorldTransform (Variables|Default|GetProjectileSpawnPoint)) "AlwaysSpawn" 0 self))
  (Utilities|IsValid _returnvalue
    (:Is%20Valid
      (Default|ActivateProjectile _returnvalue (CallFunction|GetProjectileVelocity) (Variables|Default|GetAttackDamage)))))

(event EventBeginPlay
  (|CallParentFunction))

(event EventHandleAttackSequence
  (params (SpeedRatio :type Float%20%28single-precision%29))
  ;[1 1 1] Attack Sequence : Spawn projectile
  (Utilities|Time|ClearandInvalidateTimerbyHandle (Variables|Default|GetAttackSequenceTimerHandle))
  (bind _returnvalue (Utilities|Time|SetTimerbyEvent (delegate Custom|SpawnProjectile_LocalEvent) (/ (Variables|Default|GetAttackCollisionEnableDelay) SpeedRatio)))
  (Variables|Default|SetAttackSequenceTimerHandle _returnvalue))

(fn ConstructionScript
  (|CallParentFunction))

(fn GetProjectileVelocity
  (return (* (Math|Vector|GetUnitDirection(Vector) (Transformation|GetActorLocation self) (+ (Transformation|GetActorLocation (Game|GetPlayerCharacter 0)) "0, 0,25.000000")) (Variables|Default|GetProjectileSpeed))))